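; PlayerCharacter is the player's character for what appears to be a maze game, handling movement, look input, footsteps and health.
; Movement follows the camera's forward and right vectors, and both axes feed a DoOnce that plays a footstep sound, then resets after a short delay to throttle repeats.
; Damage reduces Health, refreshes the HUD through GameModeMaze, and calls its Lose function when health runs out.
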(event `InputAxis|MoveForward`
  (params (AxisValue :type "Float (single-precision)"))
  (`self.AddMovementInput` (`KismetMathLibrary.GetForwardVector` (`SceneComponent.K2_GetComponentRotation` (`self.Camera`))) AxisValue)
  (if (!= AxisValue 0.0)
    (`/Engine/EditorBlueprintResources/StandardMacros.DoOnce` false :!label _label
      (:`Completed`
        (`GameplayStatics.PlaySoundAtLocation` "/Game/Audio/SFX/Footstep_SFX.Footstep_SFX" (`self.K2_GetActorLocation`) (struct) 1.0 1.0 0.0 null null null)
        (`KismetSystemLibrary.Delay` 0.5)
        (goto _label :!via `Reset`)))))

(event `InputAxis|MoveRight`
  (params (AxisValue :type "Float (single-precision)"))
  (`self.AddMovementInput` (`KismetMathLibrary.GetRightVector` (`SceneComponent.K2_GetComponentRotation` (`self.Camera`))) AxisValue)
  (if (!= AxisValue 0.0)
    (goto _label)))

(event `InputAxis|LookUp`
  (params (AxisValue :type "Float (single-precision)"))
  (`self.AddControllerPitchInput` AxisValue))

(event `InputAxis|Turn`
  (params (AxisValue :type "Float (single-precision)"))
  (`self.AddControllerYawInput` AxisValue))

(event `self.ReceiveAnyDamage`
  (params (Damage :type "Float (single-precision)") (DamageType :type "DamageType Object Reference") (InstigatedBy :type "Controller Object Reference") (DamageCauser :type "Actor Object Reference"))
  (set `self.health` (- (`self.health`) (`KismetMathLibrary.FTrunc` Damage)))
  (bind _asgame_mode_maze (cast `/Game/Blueprints/GameSettings/GameModeMaze` (`GameplayStatics.GetGameMode`)))
  (`/Game/UI/HUD.UpdateHealth` (`/Game/Blueprints/GameSettings/GameModeMaze.HUDWidget` _asgame_mode_maze))
  (if (<= (`self.health`) 0)
    (`/Game/Blueprints/GameSettings/GameModeMaze.Lose` _asgame_mode_maze)))

(fn `UserConstructionScript`)